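; Enemy AI controller that runs a roam-patrol behavior tree and tracks the player through AI Perception.
; Sight and hearing handlers write target and location blackboard keys and play spotted or heard-something sounds.
; Tick polls perception, clearing the last sensed location whenever the player is unperceived.
; A retriggerable delay, refreshed while the player is perceived, later clears the last known location and plays a totally-lost sound.
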(event `self.ReceiveTick`
  (params (DeltaSeconds :type "Float (single-precision)"))
  (bind _returnvalue (`GameplayStatics.GetPlayerCharacter` 0))
  (bind _aiperception (`self.AIPerception`))
  (bind _returnvalue_2 (or (`KismetArrayLibrary.Array_Contains` (`AIPerceptionComponent.GetKnownPerceivedActors` _aiperception "/Script/AIModule.AISense_Hearing") _returnvalue) (`KismetArrayLibrary.Array_Contains` (`AIPerceptionComponent.GetKnownPerceivedActors` _aiperception "/Script/AIModule.AISense_Sight") _returnvalue)))
  (`|ExecutionSequence`
    (:`then_0`
      (if (not _returnvalue_2)
        (`BlackboardComponent.ClearValue` (`AIBlueprintHelperLibrary.GetBlackboard` null) "LastSensedLoc")
        (set `self.playerGone` true)))
    (:`then_1`
      (if _returnvalue_2
        (`KismetSystemLibrary.RetriggerableDelay` 20.0)
        (if (not _returnvalue_2)
          (`BlackboardComponent.ClearValue` (`AIBlueprintHelperLibrary.GetBlackboard` null) "LastKnownLoc")
          (`GameplayStatics.PlaySoundAtLocation` "/Game/Audio/enemy_totally_lost.enemy_totally_lost" (`self.K2_GetActorLocation` (`ActorComponent.GetOwner` (`self.AIPerception`))) (struct) 1.5 1.0 0.0 "/USDCore/USDDefaultAttenuation.USDDefaultAttenuation" null null null))))))

(event `self.ReceiveBeginPlay`
  (`self.RunBehaviorTree` "/Game/Blueprints/eTP2/trees/behav_roam_patrol.behav_roam_patrol"))

(event `self.AIPerception.OnTargetPerceptionUpdated`
  (params (Actor :type "Actor Object Reference") (Stimulus :type "AIStimulus Structure"))
  (`self.handleSight` Actor Stimulus)
  (`self.handleHearing` Actor Stimulus))

(fn `handleHearing`
  (params (actor :type "Actor Object Reference") (stimulus :type "AIStimulus Structure"))
  (bind (_age _expirationage _strength _stimuluslocation _receiverlocation _tag _bsuccessfullysensed) (break `AIStimulus` stimulus))
  (bind _returnvalue (`AIBlueprintHelperLibrary.GetBlackboard` null))
  (bind _returnvalue_2 (`AIPerceptionSystem.GetSenseClassForStimulus` stimulus))
  (if (== _returnvalue_2 "/Script/AIModule.AISense_Hearing")
    (if _bsuccessfullysensed
      (`BlackboardComponent.SetValueAsVector` (`AIBlueprintHelperLibrary.GetBlackboard` null) "LastSensedLoc" _stimuluslocation)
      (if (`AIBlueprintHelperLibrary.IsValidAILocation` (`BlackboardComponent.GetValueAsVector` _returnvalue "LastSeenLoc"))
        _
        (elif (`AIBlueprintHelperLibrary.IsValidAILocation` (`BlackboardComponent.GetValueAsVector` _returnvalue "LastKnownLoc"))
          (`BlackboardComponent.SetValueAsVector` _returnvalue "LastKnownLoc" _stimuluslocation)
          (else
            (`BlackboardComponent.SetValueAsVector` _returnvalue "LastKnownLoc" _stimuluslocation)
            (`GameplayStatics.PlaySoundAtLocation` "/Game/Audio/Heard_something.Heard_something" _receiverlocation (struct) 3.0 1.0 0.0 "/USDCore/USDDefaultAttenuation.USDDefaultAttenuation" null null null)))))
    (else
      (return))))

(fn `handleSight`
  (params (Actor :type "Actor Object Reference") (Stimulus :type "AIStimulus Structure"))
  (bind (_age _expirationage _strength _stimuluslocation _receiverlocation _tag _bsuccessfullysensed) (break `AIStimulus` Stimulus))
  (bind _returnvalue (`AIBlueprintHelperLibrary.GetBlackboard` null))
  (bind _returnvalue_2 (`AIPerceptionSystem.GetSenseClassForStimulus` Stimulus))
  (if (== _returnvalue_2 "/Script/AIModule.AISense_Sight")
    (if (== (`local.Actor`) (`GameplayStatics.GetPlayerCharacter` 0))
      (`BlackboardComponent.SetValueAsObject` (`AIBlueprintHelperLibrary.GetBlackboard` null) "TargetActor" (`KismetMathLibrary.SelectObject` (`GameplayStatics.GetPlayerCharacter` 0) null _bsuccessfullysensed))
      (if _bsuccessfullysensed
        (set `self.seePlayer` true)
        (if (`self.playerGone`)
          (`GameplayStatics.PlaySoundAtLocation` "/Game/Audio/enemy_spotted.enemy_spotted" (`self.K2_GetActorLocation` (`ActorComponent.GetOwner` (`self.AIPerception`))) (struct) 1.0 1.0 0.0 "/USDCore/USDDefaultAttenuation.USDDefaultAttenuation" null null null)
          (set `self.playerGone` false))
        (else
          (set `self.seePlayer` false)))
      (if _bsuccessfullysensed
        (`BlackboardComponent.SetValueAsVector` _returnvalue "LastSensedLoc" _stimuluslocation)
        (`BlackboardComponent.SetValueAsVector` _returnvalue "LastKnownLoc" _stimuluslocation))
      (else
        (return)))
    (else
      (return))))

(fn `UserConstructionScript`)